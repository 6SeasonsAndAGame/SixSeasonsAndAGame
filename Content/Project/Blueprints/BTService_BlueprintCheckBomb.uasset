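; Behavior tree service that tells an AI character whether a bomb is available for it to interact with and where that bomb is.
; Each tick it shuffles the game state's bomb list and, skipping two bomb states, XORs each bomb's state with the pawn's team to set the interact key.
; Eligible bombs write an offset location to the blackboard.
; The loop never breaks, so later bombs overwrite earlier results.
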(event EventReceiveTickAI
  (params (OwnerController :type AI%20Controller%20Object%20Reference) (ControlledPawn :type Pawn%20Object%20Reference) (DeltaSeconds :type Float%20%28single-precision%29))
  (bind _asbp_base_character (Utilities|Casting|CastToBP_BaseCharacter ControlledPawn))
  (bind _asfps_rush_gs (Utilities|Casting|CastToFPS_Rush_GS (Game|GetGameState)))
  (Utilities|Array|Shuffle (Variables|/Game/FPS/Blueprints/Game/Rush/FPS_Rush_GS.FPS_Rush_GS_C|GetBombRef _asfps_rush_gs))
  (for _array_element (Variables|/Game/FPS/Blueprints/Game/Rush/FPS_Rush_GS.FPS_Rush_GS_C|GetBombRef _asfps_rush_gs)
    (Utilities|IsValid _array_element
      (:Is%20Valid
        (if (and (Utilities|Enum|NotEqual(Enum) (Variables|/Game/FPS/Blueprints/Interactables/Bomb/BP_Bomb.BP_Bomb_C|GetBombState _array_element) "NewEnumerator3") (Utilities|Enum|NotEqual(Enum) (Variables|/Game/FPS/Blueprints/Interactables/Bomb/BP_Bomb.BP_Bomb_C|GetBombState _array_element) "NewEnumerator2"))
          (Class|BTFunctionLibrary|SetBlackboardValueasBool (Variables|Default|GetInteractBombKey) (Class|KismetMathLibrary|XORBoolean (Utilities|Enum|Equal(Enum) (Variables|/Game/FPS/Blueprints/Interactables/Bomb/BP_Bomb.BP_Bomb_C|GetBombState _array_element) "NewEnumerator1") (Variables|/Game/FPS/Blueprints/CharacterAndClasses/BP_BaseCharacter.BP_BaseCharacter_C|GetbPawnTeam _asbp_base_character)))
          (if (Class|KismetMathLibrary|XORBoolean (Utilities|Enum|Equal(Enum) (Variables|/Game/FPS/Blueprints/Interactables/Bomb/BP_Bomb.BP_Bomb_C|GetBombState _array_element) "NewEnumerator1") (Variables|/Game/FPS/Blueprints/CharacterAndClasses/BP_BaseCharacter.BP_BaseCharacter_C|GetbPawnTeam _asbp_base_character))
            (AI|BehaviorTree|SetBlackboardValueasVector (Variables|Default|GetLocationKey) (Math|Vector|MakeVector (+ (.x (Transformation|GetActorLocation _array_element)) 1e+02) (.y (Transformation|GetActorLocation _array_element)) (.z (Transformation|GetActorLocation _array_element))))))))))