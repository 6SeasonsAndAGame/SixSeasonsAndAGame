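; Magazine is an ammo pickup that adds bullets to a character on overlap.
; When a BP_BaseCharacter enters its Sphere, it loops the character's Magazines array for entries matching its AmmoType.
; An entry below its max gains MagazineBullets without clamping, then the character updates its total bullets and the pickup destroys itself.
; The pickup stays in place when no matching entry has room.
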(event OnComponentBeginOverlap(Sphere)
  (params (OverlappedComponent :type Primitive%20Component%20Object%20Reference) (OtherActor :type Actor%20Object%20Reference) (OtherComp :type Primitive%20Component%20Object%20Reference) (OtherBodyIndex :type Integer) (bFromSweep :type Boolean) (SweepResult :type Hit%20Result%20Structure%20%28by%20ref%29))
  (bind _ammotype (Variables|Default|GetAmmoType))
  ;[1 1 1] On overlap add the magazine to the actor and destroy the magazine
  (bind _asbp_base_character (Utilities|Casting|CastToBP_BaseCharacter OtherActor))
  (for (_array_element _array_index) (Variables|/Game/Project/Blueprints/BP_BaseCharacter.BP_BaseCharacter_C|GetMagazines _asbp_base_character)
    (if (Utilities|Enum|Equal(Enum) (.ammotype _array_element) _ammotype)
      (if (< (.quantity _array_element) (.maxquantity _array_element))
        (Utilities|Array|SetArrayElem (Variables|/Game/Project/Blueprints/BP_BaseCharacter.BP_BaseCharacter_C|GetMagazines _asbp_base_character) _array_index (Utilities|Struct|MakeAmmoMagazines _ammotype (+ (.quantity _array_element) (Variables|Default|GetMagazineBullets)) (.maxquantity _array_element)))
        (Default|UpdateTotalBullets _asbp_base_character)
        (Actor|DestroyActor)))))

(fn ConstructionScript)