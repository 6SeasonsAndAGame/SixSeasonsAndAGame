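; Behavior Tree service that gives an AI pawn the location of a randomly chosen other character.
; On each tick it gathers all BP_BaseCharacter actors, and FindPlayers filters out the controlled pawn.
; It writes a random entry's location to a vector Blackboard key, as a position rather than an actor reference.
; The random index is rolled separately for the validity check and the location read.
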(event EventReceiveTickAI
  (params (OwnerController :type AI%20Controller%20Object%20Reference) (ControlledPawn :type Pawn%20Object%20Reference) (DeltaSeconds :type Float%20%28single-precision%29))
  (bind _outactors (Actor|GetAllActorsOfClass "/Game/FPS/Blueprints/CharacterAndClasses/BP_BaseCharacter.BP_BaseCharacter_C"))
  (bind _enemies (CallFunction|FindPlayers ControlledPawn _outactors))
  (if (Utilities|Array|IsValidIndex _enemies)
    (Utilities|IsValid (Utilities|Array|Get(acopy) _enemies (Math|Random|RandomIntegerinRange 0 (- (Utilities|Array|Length _enemies) 1)))
      (:Is%20Valid
        (AI|BehaviorTree|SetBlackboardValueasVector (Variables|Default|GetVectorkey) (Transformation|GetActorLocation (Utilities|Array|Get(acopy) _enemies (Math|Random|RandomIntegerinRange 0 (- (Utilities|Array|Length _enemies) 1)))))))))

(fn FindPlayers
  (params (SelfPawn :type Pawn%20Object%20Reference) (PossibleEnemies :type Array%20of%20BP%20Base%20Character%20Object%20References))
  (Utilities|Array|Clear (LocalVariables|GetEnemiesArray))
  (for _array_element PossibleEnemies
    (if (!= _array_element (.AsBP%20Base%20Character (Utilities|Casting|CastToBP_BaseCharacter SelfPawn)))
      (Utilities|Array|AddUnique (LocalVariables|GetEnemiesArray) _array_element)))
  (return (LocalVariables|GetEnemiesArray)))