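; Base flag actor for capture-the-flag, handling pickup, return and scoring on server-side capsule overlaps.
; An enemy character takes the untaken flag, which attaches to its mesh's FlagSocket.
; A teammate's touch scores team and player points if they carry a flag and this one is near its spawn, sending the carried flag home; otherwise this flag returns to spawn.
; Both teammate outcomes briefly deactivate this flag through a delayed reset.
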(event OnComponentBeginOverlap(Capsule)
  (params (OverlappedComponent :type Primitive%20Component%20Object%20Reference) (OtherActor :type Actor%20Object%20Reference) (OtherComp :type Primitive%20Component%20Object%20Reference) (OtherBodyIndex :type Integer) (bFromSweep :type Boolean) (SweepResult :type Hit%20Result%20Structure%20%28by%20ref%29))
  ;[0.01562 0.01562 0.01562] OnOverlap with flag capsule
  (Networking|SwitchHasAuthority
    (:Authority
      (if (Variables|Default|GetbActive)
        (if (not (Variables|Default|GetbFlagTaken))
          (bind _asbp_base_character (Utilities|Casting|CastToBP_BaseCharacter OtherActor))
          (bind _output_get (Variables|Default|SetPawnRef _asbp_base_character))
          (if (not (Variables|/Game/Project/Blueprints/BP_BaseCharacter.BP_BaseCharacter_C|GetbDead _output_get))
            (if (not (Math|Boolean|Equal(Boolean) (Variables|/Game/Project/Blueprints/BP_BaseCharacter.BP_BaseCharacter_C|GetbPawnTeam _asbp_base_character) (Variables|Default|GetTeam)))
              (if (not (Variables|/Game/Project/Blueprints/BP_BaseCharacter.BP_BaseCharacter_C|GetbCarringFlag (Variables|Default|GetPawnRef)))
                (Default|ServeronPickupFlag (Variables|Default|GetPawnRef) self)
                (Variables|Default|SetbFlagTaken true)
                (Utilities|IsValid (Variables|Default|GetPawnRef)
                  (:Is%20Valid
                    (Transformation|AttachComponentToComponent (Variables|/Script/Engine.Character|GetMesh (Variables|Default|GetPawnRef)) "FlagSocket" "SnapToTarget" "KeepRelative" "KeepRelative" true))))
              (else
                ;;[1 1 1] Your Team flag
                (bind _success (CallFunction|TrytoAddPoint))
                (if _success
                  (Utilities|FlowControl|Delay 0.2)
                  (Utilities|IsValid (Variables|Default|GetPawnRef)
                    (:Is%20Valid
                      (Default|ServeronDropFlag (Variables|Default|GetPawnRef)))
                    (:Is%20Not%20Valid
                      _))
                  (Variables|Default|SetbFlagTaken false))))))))))

(event Custom|ResetFlag
  ;[0.01562 0.01562 0.01562] OnOverlap with flag capsule
  (Utilities|FlowControl|Delay 1.0)
  (Variables|Default|SetbActive true))

(event EventBeginPlay
  ;[1 0.2273 0.1175] BeginPlay
  (Networking|SwitchHasAuthority
    (:Authority
      (Variables|Default|SetInitialPossition (Transformation|GetActorLocation))
      (Variables|Default|SetInitialRotation (Transformation|GetActorRotation)))))

(fn ConstructionScript)

(fn TrytoAddPoint
  (bind _pawnref (Variables|Default|GetPawnRef))
  (bind _pawnref_2 (Variables|Default|GetPawnRef))
  (bind _flagref (Variables|/Game/Project/Blueprints/BP_BaseCharacter.BP_BaseCharacter_C|GetFlagRef _pawnref))
  (if (and (Variables|/Game/Project/Blueprints/BP_BaseCharacter.BP_BaseCharacter_C|GetbCarringFlag (Variables|Default|GetPawnRef)) (<= (Math|Float|Absolute(Float) (Math|Vector|VectorLength (- (Variables|Default|GetInitialPossition) (Transformation|GetActorLocation)))) 2e+02))
    ;[1 1 1] Add points
    (bind _asfps_ctf_gs (Utilities|Casting|CastToFPS_CTF_GS (Game|GetGameState)))
    (Default|AddTeamPoints _asfps_ctf_gs (Variables|/Game/Project/Blueprints/BP_BaseCharacter.BP_BaseCharacter_C|GetbPawnTeam _pawnref_2))
    (bind _asfps_player_state (Utilities|Casting|CastToFPS_PlayerState (Variables|/Script/Engine.Pawn|GetPlayerState _pawnref_2)))
    (Default|ServerAddScorePoints _asfps_player_state 3.5e+02 "NewEnumerator11")
    ;[1 1 1] ResetFlag
    (Variables|Default|SetbActive false)
    (Default|DropFlag _pawnref)
    (CallFunction|ResetFlag)
    (Transformation|SetActorLocation _flagref (Variables|BP_BaseFlag_C|GetInitialPossition _flagref) false true)
    (Networking|ForceNetUpdate)
    (return true)
    (else
      (Variables|Default|SetbActive false)
      (CallFunction|ResetFlag)
      (Transformation|Teleport (Variables|Default|GetInitialPossition) (Variables|Default|GetInitialRotation))
      (Transformation|SetActorRotation "0, 0, 0" true)
      (return false))))