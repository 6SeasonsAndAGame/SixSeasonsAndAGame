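; Behavior tree service that tells an AI pawn whether it has a clear shot at its blackboard enemy.
; Each tick it line-traces between both characters at raised height on TraceTypeQuery4, setting the CanShoot key true when nothing blocks.
; A FindEnemy function, not called by the tick, returns the nearest opposing-team character confirmed by a visibility trace, despite its input being named CapturePoints.
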(event EventReceiveTickAI
  (params (OwnerController :type AI%20Controller%20Object%20Reference) (ControlledPawn :type Pawn%20Object%20Reference) (DeltaSeconds :type Float%20%28single-precision%29))
  (bind _returnvalue (Transformation|GetActorLocation ControlledPawn))
  (bind _enemykey (Variables|Default|GetEnemyKey))
  (bind _returnvalue_2 (Class|BTFunctionLibrary|GetBlackboardValueasObject _enemykey))
  (bind _asbp_base_character (Utilities|Casting|CastToBP_BaseCharacter _returnvalue_2))
  (bind _returnvalue_3 (Transformation|GetActorLocation _asbp_base_character))
  (Utilities|IsValid _returnvalue_2
    (:Is%20Valid
      (bind _outhit (Collision|LineTraceByChannel (Math|Vector|MakeVector (.x _returnvalue) (.y _returnvalue) (+ (.z _returnvalue) 8e+01)) (Math|Vector|MakeVector (.x _returnvalue_3) (.y _returnvalue_3) (+ (.z _returnvalue_3) 8e+01)) "TraceTypeQuery4" false (Utilities|Array|MakeArray ControlledPawn) "None"))
      (Class|BTFunctionLibrary|SetBlackboardValueasBool (Variables|Default|GetCanShootKey) (not (.bblockinghit _outhit))))))

(fn FindEnemy
  (params (CapturePoints :type Array%20of%20BP%20Base%20Character%20Object%20References) (SelfPawn :type Pawn%20Object%20Reference))
  (Utilities|Array|Clear (Variables|Default|GetPosibleEnemies))
  (LocalVariables|SetMinDistance 2.5e+05)
  (LocalVariables|SetPawn SelfPawn)
  (for _array_element CapturePoints
    (if (Math|Boolean|NotEqual(Boolean) (Variables|/Game/FPS/Blueprints/CharacterAndClasses/BP_BaseCharacter.BP_BaseCharacter_C|GetbPawnTeam (.AsBP%20Base%20Character (Utilities|Casting|CastToBP_BaseCharacter (LocalVariables|GetPawn)))) (Variables|/Game/FPS/Blueprints/CharacterAndClasses/BP_BaseCharacter.BP_BaseCharacter_C|GetbPawnTeam _array_element))
      (bind _outhit (Collision|LineTraceByChannel (Transformation|GetActorLocation (LocalVariables|GetPawn)) (Transformation|GetActorLocation _array_element) "TraceTypeQuery1" false 0 "None"))
      (bind _asbp_base_character (Utilities|Casting|CastToBP_BaseCharacter (.hitactor _outhit)))
      (if (== _asbp_base_character _array_element)
        (Utilities|Array|Add (Variables|Default|GetPosibleEnemies) _array_element))))
  (if (!= (Utilities|Array|Length (Variables|Default|GetPosibleEnemies)) 0)
    ;[1 1 1] Find The closest
    (for _array_element_2 (Variables|Default|GetPosibleEnemies)
      (if (< (Math|Float|Absolute(Float) (Math|Vector|VectorLength (- (Transformation|GetActorLocation _array_element_2) (Transformation|GetActorLocation (LocalVariables|GetPawn))))) (LocalVariables|GetMinDistance))
        (Variables|Default|SetEnemy _array_element_2)
        (LocalVariables|SetMinDistance (Math|Float|Absolute(Float) (Math|Vector|VectorLength (- (Transformation|GetActorLocation _array_element_2) (Transformation|GetActorLocation (LocalVariables|GetPawn))))))))
    (return (Variables|Default|GetEnemy))
    (else
      (return 0))))