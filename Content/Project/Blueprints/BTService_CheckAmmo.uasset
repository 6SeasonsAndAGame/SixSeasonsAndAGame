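; Behavior tree service that tells the AI when its character needs to reload its current weapon.
; Each tick it casts the controlled pawn to BP_BaseCharacter and writes a reload blackboard bool.
; The bool is true only while the character is alive and its valid current weapon has zero ammo; a dead character or missing weapon sets it false.
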(event EventReceiveTickAI
  (params (OwnerController :type AI%20Controller%20Object%20Reference) (ControlledPawn :type Pawn%20Object%20Reference) (DeltaSeconds :type Float%20%28single-precision%29))
  (bind _breload_key (Variables|Default|GetbReload%20Key))
  (bind _asbp_base_character (Utilities|Casting|CastToBP_BaseCharacter ControlledPawn))
  (if (not (Variables|/Game/FPS/Blueprints/CharacterAndClasses/BP_BaseCharacter.BP_BaseCharacter_C|GetbDead _asbp_base_character))
    (Utilities|IsValid (Variables|/Game/FPS/Blueprints/CharacterAndClasses/BP_BaseCharacter.BP_BaseCharacter_C|GetCurrentWeapon _asbp_base_character)
      (:Is%20Valid
        (Class|BTFunctionLibrary|SetBlackboardValueasBool _breload_key (== (Variables|/Game/FPS/Blueprints/Weapons/BP_BaseWeapon.BP_BaseWeapon_C|GetActualAmmo (Variables|/Game/FPS/Blueprints/CharacterAndClasses/BP_BaseCharacter.BP_BaseCharacter_C|GetCurrentWeapon _asbp_base_character)) 0)))
      (:Is%20Not%20Valid
        (Class|BTFunctionLibrary|SetBlackboardValueasBool _breload_key false :!label _label)))
    (else
      (goto _label))))