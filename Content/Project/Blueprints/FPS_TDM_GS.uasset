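; Team deathmatch game state for an FPS mode that tracks each team's score and ends the match at the point limit.
; A server event adds one point on a kill to Team A or Team B, selected by a boolean.
; When that team's total reaches the win threshold, it casts to the FPS game mode and calls its end-game event with the winning team's flag.
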(event Custom|Server_AddTeamPoints
  (params (bTeam :type Boolean))
  ;[1 1 1] Add Points on kill
  (if bTeam
    (bind _result (Math|Integer|IncrementInt (Variables|Default|GetTeamB_Points))
      (:%20%20
        (bind _output_get (Variables|Default|SetTeamB_Points _result))
        (if (>= _output_get (Variables|Default|GetPointsToWin))
          (bind _asfps_gm (Utilities|Casting|CastToFPS_GM (Game|GetGameMode)))
          (Default|ServerEndGame _asfps_gm true))))
    (else
      (bind _result_2 (Math|Integer|IncrementInt (Variables|Default|GetTeamA_Points))
        (:%20%20
          (bind _output_get_2 (Variables|Default|SetTeamA_Points _result_2))
          (if (>= _output_get_2 (Variables|Default|GetPointsToWin))
            (bind _asfps_gm_2 (Utilities|Casting|CastToFPS_GM (Game|GetGameMode)))
            (Default|ServerEndGame _asfps_gm_2 false)))))))

(fn ConstructionScript)