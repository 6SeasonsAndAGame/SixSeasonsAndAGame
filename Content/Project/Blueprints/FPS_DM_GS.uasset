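; Deathmatch game state that tracks the player with the most kills and ends the match at a kill target.
; On authority, BeginPlay runs one update: it scans PlayerArray for the leader, then after a short delay compares that leader's kills to PointsToWin.
; Reaching the target calls ServerEndDeathmatch on FPS_DM_GM, forces a net update and clears UpdateWinnerTimer, which is not set in these graphs.
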(event Custom|UpdateGameState
  ;[1 1 1] Update Game State
  (CallFunction|UpdateWinner)
  (Utilities|FlowControl|Delay 0.5)
  (CallFunction|CheckWinnerPoints))

(event EventBeginPlay
  ;[1 1 1] BeginPlay
  (|CallParentFunction)
  (Networking|SwitchHasAuthority
    (:Authority
      (CallFunction|UpdateGameState))))

(fn ConstructionScript
  (|CallParentFunction))

(fn CheckWinnerPoints
  (bind _actualwinner (Variables|Default|GetActualWinner)
    (:then
      (if (>= (Variables|/Game/Project/Blueprints/FPS_PlayerState.FPS_PlayerState_C|GetKills _actualwinner) (Variables|Default|GetPointsToWin))
        (bind _asfps_dm_gm (Utilities|Casting|CastToFPS_DM_GM (Game|GetGameMode)))
        (Default|ServerEndDeathmatch _asfps_dm_gm)
        (Networking|ForceNetUpdate)
        (Utilities|Time|ClearandInvalidateTimerbyHandle (Variables|Default|GetUpdate%20WinnerTimer))))
    (:else)))

(fn UpdateWinner
  (for _array_element (Variables|Default|GetPlayerArray)
    (bind _asfps_player_state (Utilities|Casting|CastToFPS_PlayerState _array_element))
    (bind _actualwinner (Variables|Default|GetActualWinner)
      (:then
        (if (> (Variables|/Game/Project/Blueprints/FPS_PlayerState.FPS_PlayerState_C|GetKills _asfps_player_state) (Variables|/Game/Project/Blueprints/FPS_PlayerState.FPS_PlayerState_C|GetKills _actualwinner))
          (Variables|Default|SetActualWinner _asfps_player_state :!label _label)
          (Networking|ForceNetUpdate)))
      (:else
        (goto _label)))))