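; BP_PopPop is an interactable actor, apparently a vending machine, that plays a "Pop Pop" sound on F.
; The F press plays the sound at the Box location and prints "Pop Pop".
; Box begin overlap enables input on a BP_BaseCharacter cast from the overlapping actor's owner.
; End overlap instead casts that owner to FPS_TDM_GM to disable input, and neither call targets this actor.
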(event OnComponentBeginOverlap(Box)
  (params (OverlappedComponent :type Primitive%20Component%20Object%20Reference) (OtherActor :type Actor%20Object%20Reference) (OtherComp :type Primitive%20Component%20Object%20Reference) (OtherBodyIndex :type Integer) (bFromSweep :type Boolean) (SweepResult :type Hit%20Result%20Structure%20%28by%20ref%29))
  (bind _asbp_base_character (Utilities|Casting|CastToBP_BaseCharacter (Components|GetOwner OtherActor)))
  (Input|EnableInput _asbp_base_character (Game|GetPlayerController (stale OnComponentEndOverlap(Box) OtherBodyIndex))))

(event OnComponentEndOverlap(Box)
  (params (OverlappedComponent :type Primitive%20Component%20Object%20Reference) (OtherActor :type Actor%20Object%20Reference) (OtherComp :type Primitive%20Component%20Object%20Reference) (OtherBodyIndex :type Integer))
  (bind _asfps_tdm_gm (Utilities|Casting|CastToFPS_TDM_GM (Components|GetOwner OtherActor)))
  (Input|DisableInput _asfps_tdm_gm (Game|GetPlayerController OtherBodyIndex)))

(event Input|KeyboardEvents|F
  (params (Key :type Key%20Structure))
  (:Pressed
    (Audio|PlaySoundatLocation "/Game/Audio/Pop_pop_vending_machine_draft_no_mod.Pop_pop_vending_machine_draft_no_mod" (Transformation|GetWorldLocation (Variables|Default|GetBox)) "0, 0, 0" 1.0 1.0 0.0 0 0 0)
    (Development|PrintString "Pop Pop")))

(fn ConstructionScript)