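; Behavior tree service for Conquest AI that points the controlled pawn at the nearest capture point its team can target.
; Each tick it gathers all BP_ConquestCapturePoint actors and keeps those whose FlagState qualifies for the pawn's boolean PawnTeam.
; It writes the closest one's location to a vector Blackboard key, leaving the key untouched when none qualify.
; An older filter using Active and HolderTeam remains disconnected.
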(event EventReceiveTickAI
  (params (OwnerController :type AI%20Controller%20Object%20Reference) (ControlledPawn :type Pawn%20Object%20Reference) (DeltaSeconds :type Float%20%28single-precision%29))
  (bind _outactors (Actor|GetAllActorsOfClass "/Game/FPS/Blueprints/Misc/ConquestZones/BP_ConquestCapturePoint.BP_ConquestCapturePoint_C"))
  (if (Utilities|Array|IsValidIndex _outactors)
    (bind _flag (CallFunction|FindClosestFlag _outactors ControlledPawn))
    (Utilities|IsValid _flag
      (:Is%20Valid
        (AI|BehaviorTree|SetBlackboardValueasVector (Variables|Default|GetVectorkey) (Transformation|GetActorLocation _flag))))))

(fn FindClosestFlag
  (params (CapturePoints :type Array%20of%20BP%20Conquest%20Capture%20Point%20Object%20References) (SelfPawn :type Pawn%20Object%20Reference))
  (Utilities|Array|Clear (Variables|Default|GetPosibleFlagsToCapture))
  (LocalVariables|SetMinDistance 2.5e+05)
  (LocalVariables|SetPawn SelfPawn)
  (for _array_element CapturePoints
    (if (Utilities|Enum|Equal(Enum) (Variables|/Game/FPS/Blueprints/Misc/ConquestZones/BP_ConquestCapturePoint.BP_ConquestCapturePoint_C|GetFlagState _array_element) "NewEnumerator2")
      (Utilities|Array|Add (Variables|Default|GetPosibleFlagsToCapture) _array_element :!label _label)
      (elif (Variables|/Game/FPS/Blueprints/CharacterAndClasses/BP_BaseCharacter.BP_BaseCharacter_C|GetbPawnTeam (.AsBP%20Base%20Character (Utilities|Casting|CastToBP_BaseCharacter (LocalVariables|GetPawn))))
        (if (Utilities|Enum|Equal(Enum) (Variables|/Game/FPS/Blueprints/Misc/ConquestZones/BP_ConquestCapturePoint.BP_ConquestCapturePoint_C|GetFlagState _array_element) "NewEnumerator0")
          (goto _label))
        (elif (Utilities|Enum|Equal(Enum) (Variables|/Game/FPS/Blueprints/Misc/ConquestZones/BP_ConquestCapturePoint.BP_ConquestCapturePoint_C|GetFlagState _array_element) "NewEnumerator1")
          (goto _label)))))
  (if (!= (Utilities|Array|Length (Variables|Default|GetPosibleFlagsToCapture)) 0)
    ;[1 1 1] Find The closest
    (for _array_element_2 (Variables|Default|GetPosibleFlagsToCapture)
      (if (< (Math|Float|Absolute(Float) (Math|Vector|VectorLength (- (Transformation|GetActorLocation _array_element_2) (Transformation|GetActorLocation (LocalVariables|GetPawn))))) (LocalVariables|GetMinDistance))
        (Variables|Default|SetFlag _array_element_2)
        (LocalVariables|SetMinDistance (Math|Float|Absolute(Float) (Math|Vector|VectorLength (- (Transformation|GetActorLocation _array_element_2) (Transformation|GetActorLocation (LocalVariables|GetPawn))))))))
    (return (Variables|Default|GetFlag))
    (else
      (return 0))))