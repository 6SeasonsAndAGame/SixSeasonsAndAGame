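; BP_SimpleVehicle is a drivable four-wheeled vehicle Blueprint for the FPS game.
; The MoveForward and MoveRight axes feed throttle and steering into its WheeledVehicleMovementComponent4W.
; Space Bar, bound directly as a key event, engages the handbrake while held.
; BeginPlay and the construction script only call their parent versions.
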(event EventBeginPlay
  (|CallParentFunction))

(event Input|AxisEvents|InputAxisMoveForward
  (params (AxisValue :type Float%20%28single-precision%29))
  ;[1 1 1] Throttle input
  (Class|WheeledVehicleMovementComponent|SetThrottleInput (Variables|Default|GetWheeledVehicleMovementComponent4W) AxisValue))

(event Input|AxisEvents|InputAxisMoveRight
  (params (AxisValue :type Float%20%28single-precision%29))
  (Class|WheeledVehicleMovementComponent|SetSteeringInput (Variables|Default|GetWheeledVehicleMovementComponent4W) AxisValue))

(event Input|KeyboardEvents|SpaceBar
  (params (Key :type Key%20Structure :default "None"))
  (bind _wheeledvehiclemovementcomponent4w (Variables|Default|GetWheeledVehicleMovementComponent4W))
  (:Pressed
    (Class|WheeledVehicleMovementComponent|SetHandbrakeInput _wheeledvehiclemovementcomponent4w true))
  (:Released
    (Class|WheeledVehicleMovementComponent|SetHandbrakeInput _wheeledvehiclemovementcomponent4w false)))

(fn ConstructionScript
  (|CallParentFunction))