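; LobbyPC is the player controller for the FPS lobby, handling each player's lobby menu, name, ready state and map vote.
; Client events create the WB_Lobby widget with UI-only input, rebuild its player list from passed-in info, and remove widgets.
; Server events set name and ready state in PlayerInfo, then have FPS_Lobby_GM update everyone.
; Map votes pass to the game mode, limited to one by CanVote.
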(event Custom|Server_CallUpdate
  ;[1 1 1] Call Update
  (bind _asfps_lobby_gm (Utilities|Casting|CastToFPS_Lobby_GM (Game|GetGameMode)))
  (Default|MulticastEveryoneUpdate _asfps_lobby_gm))

(event Custom|Client_InitialSetUp
  ;[1 1 1] Init
  (CallFunction|ServerSetPlayerName self)
  (CallFunction|ServerCallUpdate))

(event Custom|Client_SetupLobbyMenu
  ;[1 1 1] Open Lobby Menu
  (Variables|Default|SetbShowMouseCursor true)
  (bind _returnvalue (UserInterface|CreateWidget "/Game/FPS/IntroScreen/Lobby/WB_Lobby.WB_Lobby_C" (Game|GetPlayerController 0)))
  (bind _output_get (Variables|Default|SetLobbyRef _returnvalue))
  (UserInterface|Viewport|AddtoViewport _output_get 0)
  (Input|SetInputModeUIOnly self _output_get "DoNotLock"))

(event Custom|Server_VoteMap
  (params (Map :type Integer))
  ;[1 1 1] Vote Map
  (if (Variables|Default|GetbCanVote)
    (Variables|Default|SetbCanVote false)
    (bind _asfps_lobby_gm (Utilities|Casting|CastToFPS_Lobby_GM (Game|GetGameMode)))
    (Default|ServerIncreaseMapVotes _asfps_lobby_gm Map)))

(event Custom|Client_AddPlayerToTheList
  (params (NewParam :type Array%20of%20Lobby%20Player%20Info%20Structures))
  (bind _lobbyref (Variables|Default|GetLobbyRef))
  ;[1 1 1] Print Player List
  (Utilities|IsValid _lobbyref
    (:Is%20Valid
      (Default|ClearPlayerList _lobbyref)
      (for _array_element NewParam
        (bind _returnvalue (UserInterface|CreateWidget "/Game/FPS/IntroScreen/Lobby/PlayerInLobby.PlayerInLobby_C" self _array_element))
        (Class|VerticalBox|AddChildtoVerticalBox (Variables|/Game/FPS/IntroScreen/Lobby/WB_Lobby.WB_Lobby_C|GetPlayerList (Variables|Default|GetLobbyRef)) _returnvalue)))))

(event Custom|Server_SetPlayerName
  (params (LobbyPC :type Lobby%20PC%20Object%20Reference))
  ;[1 1 1] Set Name/State
  (Variables|LobbyPC_C|SetPlayerInfo LobbyPC (Utilities|Struct|MakeLobbyPlayerInfo (Utilities|Text|ToText(String) (PlayerState|GetPlayerName (Variables|GetPlayerState))) false)))

(event Custom|Server_ToggleReady
  ;[1 1 1] ToggleReady State
  (Variables|Default|SetPlayerInfo (Utilities|Struct|MakeLobbyPlayerInfo (.name (Variables|Default|GetPlayerInfo)) (not (.bready (Variables|Default|GetPlayerInfo)))))
  (CallFunction|ServerCallUpdate))

(event Custom|Client_RemoveWidget
  ;[1 1 1] Remove Widget
  (Viewport|RemoveAllWidgets))

(fn ConstructionScript)