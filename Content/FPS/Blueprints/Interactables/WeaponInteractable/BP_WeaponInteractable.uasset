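; Interactable weapon pickup that hands its weapon class, with a fixed ammo count, to the interacting BP_BaseCharacter, then tears off and destroys itself.
; On BeginPlay it disables mesh collision, then after a long delay shows the mesh and restores collision.
; Replication of WeaponToSpawn also shows the mesh and applies a random rotation.
; Logic for physics and per-weapon mesh materials is unconnected, and BeginHover just returns false.
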(event Custom|ShowMesh
  ;[1 1 1] Begin Play
  (Rendering|SetVisibility (Variables|Default|GetStaticMesh) true false))

(event EventBeginPlay
  (Collision|SetCollisionEnabled (Variables|Default|GetStaticMesh) "NoCollision")
  (Utilities|FlowControl|Delay 1.2e+02)
  (CallFunction|ShowMesh)
  (Collision|SetCollisionEnabled (Variables|Default|GetStaticMesh) "QueryAndPhysics"))

(event Collision|EventActorBeginOverlap
  (params (OtherActor :type Actor%20Object%20Reference))
  (|CallParentFunction OtherActor) ; This node is disabled and will not be called.\nDrag off pins to build functionality.
)

(event EventTick
  (params (DeltaSeconds :type Float%20%28single-precision%29))
  (|CallParentFunction DeltaSeconds) ; This node is disabled and will not be called.\nDrag off pins to build functionality.
)

(event EventInteract
  (params (Instigator :type Actor%20Object%20Reference))
  ;[1 1 1] Interact
  (bind _asbp_base_character (Utilities|Casting|CastToBP_BaseCharacter Instigator))
  (Default|ClientPickUpWeapon _asbp_base_character (Variables|Default|GetWeaponToSpawn) 30)
  (Class|Actor|TearOff)
  (Actor|DestroyActor))

(fn ConstructionScript
  (|CallParentFunction))

(fn OnRepWeapontoSpawn
  (CallFunction|ShowMesh)
  (Transformation|SetActorRotation (Math|Random|RandomRotator false)))

(fn BeginHover
  (params (Instigator :type Actor%20Object%20Reference))
  (return false))