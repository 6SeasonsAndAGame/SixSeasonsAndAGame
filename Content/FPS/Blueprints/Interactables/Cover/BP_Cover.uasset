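; Interactable cover actor that a character attaches to, optionally crouched, and moves between left, middle and right points.
; Interaction multicasts the attach if unoccupied; point selection restarts a Tick-driven lerp that moves the player through ServerSetLocation.
; NetworkSafe events branch on authority, routing client occupancy changes through the player's server event because the client lacks ownership of the cover.
; Detaching uncrouches the player and frees the cover.
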(event Custom|SetPlayerPositionToSelectedPoint
  (params (Player :type BP%20Base%20Character%20Object%20Reference))
  ;[1 1 1] Handle Player Position
  (bind _output_get (Variables|Default|SetAttachedPlayer Player))
  (Variables|Default|SetPlayerLocationOnStartLerp (Transformation|GetWorldLocation (Variables|/Script/Engine.Actor|GetRootComponent _output_get))) ; Lerp input A & B need to be constant\nin order to have a linear interpolation
  (Variables|Default|SetLerpBetweenPoints 0.0))

(event Custom|PlayerHasDetached
  (params (Local%20Player :type BP%20Base%20Character%20Object%20Reference))
  ;[1 1 1] Detach Player
  (Default|ForceUncrouch Local%20Player)
  (CallFunction|NetworkSafeSetIsOccupiedbyPlayer false Local%20Player))

(event Custom|NetworkSafe_Interact
  (params (Instigator :type Actor%20Object%20Reference))
  ;[1 1 1] Initial Interaction
  (Networking|SwitchHasAuthority
    (:Authority
      (CallFunction|MulticastInteract Instigator))
    (:Remote
      (CallFunction|ServerInteract Instigator))))

(event Custom|LocalServerOnly_SetIsOccupiedByPlayer
  (params (Value :type Boolean))
  ;[1 1 1] Sync IsOccupiedByPlayer
  (Variables|Default|SetIsOccupiedByPlayer Value))

(event Custom|NetworkSafe_SetIsOccupiedByPlayer
  (params (Value :type Boolean) (Local%20Player :type BP%20Base%20Character%20Object%20Reference))
  ;[1 1 1] Sync IsOccupiedByPlayer
  (Networking|SwitchHasAuthority ; Authority == Server\nRemote == Client
    (:Authority
      (CallFunction|LocalServerOnlySetIsOccupiedbyPlayer Value) ; Local Server Only should only be called by the server
    )
    (:Remote
      (Default|ServerCoverSetIsOccupiedbyPlayer Local%20Player Value self) ; Server events go from client with ownership -> server
    )))

(event Custom|Multicast%20Interact
  (params (Instigator :type Actor%20Object%20Reference))
  ;[1 1 1] Initial Interaction
  (if (not (Variables|Default|GetIsOccupiedByPlayer))
    (bind _asbp_base_character (Utilities|Casting|CastToBP_BaseCharacter Instigator))
    (if (Pawn|IsLocallyControlled _asbp_base_character)
      _
      (else
        _))
    (CallFunction|SelectCoverPoint (Variables|Default|GetStartingCoverPoint))
    (CallFunction|SetPlayerPositiontoSelectedPoint _asbp_base_character)
    (Default|AttachtoCover _asbp_base_character self)
    (if (Variables|Default|GetCrouchOnStart)
      (Default|ForceCrouch _asbp_base_character))
    (CallFunction|NetworkSafeSetIsOccupiedbyPlayer true _asbp_base_character)))

(event Custom|Server_Interact
  (params (Instigator :type Actor%20Object%20Reference))
  ;[1 1 1] Initial Interaction
  (CallFunction|MulticastInteract Instigator))

(event EventTick
  (params (DeltaSeconds :type Float%20%28single-precision%29))
  ;[1 1 1] Handle Player Position
  ;;[0 0.3525 0.3849] Check that a lerp is in progress before changing player location
  (bind _output (CallFunction|Approximately (Variables|Default|GetLerpBetweenPoints) (Variables|Default|GetTimeToLerpBetweenPoints) 0.01))
  (if (not _output)
    ;;[0 0.3525 0.3849] Increase current lerp time by delta time, & clamp to target time
    (Variables|Default|SetLerpBetweenPoints (Math|Float|Clamp(Float) (+ (Variables|Default|GetLerpBetweenPoints) DeltaSeconds) 0.0 (Variables|Default|GetTimeToLerpBetweenPoints)))
    ;;[0 0.3525 0.3849] Fit the current time to a zero to a 0-1 float
    ;; & apply position  to player using Vector Lerp
    (bind _selectedcoverpoint (Variables|Default|GetSelectedCoverPoint)
      (:then
        (Variables|Default|GetAttachedPlayer
          (:then
            (bind _output_2 (CallFunction|Fitto01 (Variables|Default|GetLerpBetweenPoints) (Variables|Default|GetTimeToLerpBetweenPoints)))
            (Default|ServerSetLocation (Variables|Default|GetAttachedPlayer) (Math|Vector|Lerp(Vector) (Variables|Default|GetPlayerLocationOnStartLerp) (+ (Transformation|GetWorldLocation _selectedcoverpoint) (Variables|Default|GetVerticalPlayerLocationOffset)) _output_2)))
          (:else)))
      (:else))))

(event EventInteract
  (params (Instigator :type Actor%20Object%20Reference))
  ;[1 1 1] Initial Interaction
  (CallFunction|MulticastInteract Instigator))

(fn ConstructionScript
  (Transformation|SetRelativeLocation (Variables|Default|GetLeftPoint) (Variables|Default|GetLeftPointLocation) false false)
  (Transformation|SetRelativeLocation (Variables|Default|GetMiddlePoint) (Variables|Default|GetMiddlePointLocation) false false)
  (Transformation|SetRelativeLocation (Variables|Default|GetRightPoint) (Variables|Default|GetRightPointLocation) false false))

(fn SelectCoverPoint
  (params (CoverPoint :type ECoverPoint%20Enum :default "NewEnumerator0"))
  (switch Utilities|FlowControl|Switch|SwitchonECoverPoint CoverPoint
    (:NewEnumerator0
      (Variables|Default|SetSelectedCoverPoint (Variables|Default|GetLeftPoint))
      (Variables|Default|SetSelectedCoverPointIndex -1))
    (:NewEnumerator1
      (Variables|Default|SetSelectedCoverPoint (Variables|Default|GetMiddlePoint))
      (Variables|Default|SetSelectedCoverPointIndex 0))
    (:NewEnumerator2
      (Variables|Default|SetSelectedCoverPoint (Variables|Default|GetRightPoint))
      (Variables|Default|SetSelectedCoverPointIndex 1))))

(fn SelectCoverPointbyIndex
  (params (Index :type Integer))
  (if (== Index -1)
    (CallFunction|SelectCoverPoint "NewEnumerator0")
    (elif (== Index 0)
      (CallFunction|SelectCoverPoint "NewEnumerator1")
      (elif (== Index 1)
        (CallFunction|SelectCoverPoint "NewEnumerator2")
        (else
          (Development|PrintString "Invalid cover point index" true true "(R=1.000000,G=0.057348,B=0.000000,A=1.000000)"))))))

(fn IteratePoints
  (params (Dir :type Integer) (Instigator :type BP%20Base%20Character%20Object%20Reference))
  (bind _selectedcoverpointindex (Variables|Default|GetSelectedCoverPointIndex))
  (if (> Dir 0)
    (CallFunction|SelectCoverPointbyIndex (Math|Integer|Clamp(Integer) (+ (Variables|Default|GetSelectedCoverPointIndex) 1) -1 1))
    (else
      (CallFunction|SelectCoverPointbyIndex (Math|Integer|Clamp(Integer) (- (Variables|Default|GetSelectedCoverPointIndex) 1) -1 1))))
  (CallFunction|SetPlayerPositiontoSelectedPoint Instigator)
  (Development|PrintString (Utilities|String|ToString(Integer) _selectedcoverpointindex))
  (return _selectedcoverpointindex))

(fn BeginHover
  (params (Instigator :type Actor%20Object%20Reference))
  (return false))