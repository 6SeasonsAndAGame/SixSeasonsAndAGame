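; Interactable fire alarm that, when first used, plays a pull animation, sparks, fails critically, then falls and catches fire with sound.
; The server gates the one-time interaction and multicasts the timed animation and spark sequence.
; Tick accelerates the alarm toward a configurable local fall point, spawning fire after landing.
; The server then sets replicated AnimationComplete, whose OnRep snaps the alarm down and spawns fire for clients that missed the range-limited multicast.
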(event Custom|Multicast_Interact
  (bind _alarm (Variables|Default|GetAlarm))
  ;[1 1 1] Play Animation For All
  (Components|Animation|PlayAnimation _alarm "/Game/FPS/Assets/AnimatedProps/AlarmCriticalFailure/SM_Fake_Fire_Alarm_Animated_Anim_AlarmArm_AlarmPull.SM_Fake_Fire_Alarm_Animated_Anim_AlarmArm_AlarmPull" false)
  (Utilities|FlowControl|Delay 1.3)
  (CallFunction|SpawnSparks)
  (Utilities|FlowControl|Delay 0.2)
  (CallFunction|SpawnSparks)
  (Utilities|FlowControl|Delay 0.6)
  (Components|Animation|PlayAnimation _alarm "/Game/FPS/Assets/AnimatedProps/AlarmCriticalFailure/SM_Fake_Fire_Alarm_Animated_Anim_AlarmArm_AlarmCriticalFailure.SM_Fake_Fire_Alarm_Animated_Anim_AlarmArm_AlarmCriticalFailure" false)
  (Utilities|FlowControl|Delay 1.1)
  (Variables|Default|SetIsFalling true))

(event Custom|OnRep_AnimationCompleteEvent
  ;[1 1 1] Ensure players who were out of range for the Multicast still get synced to the current state
  (if (and (Variables|Default|GetAnimationComplete) (not (Variables|Default|GetIsFalling)))
    (Transformation|SetRelativeLocation (Variables|Default|GetAlarm) (Variables|Default|GetFallPointLocalPosition) false false)
    (CallFunction|SpawnFire)))

(event Custom|SpawnFire
  (bind _alarm (Variables|Default|GetAlarm))
  (bind _returnvalue (Transformation|GetWorldLocation _alarm))
  ;[1 1 1] Particle Events
  (Effects|SpawnEmitteratLocation "/Game/M5VFXVOL2/Particles/Fire/Fire_00.Fire_00" _returnvalue "0, 0, 0" "1.000000,1.000000,1.000000" false)
  (Class|AkGameplayStatics|PostEventatLocation "/Game/WwiseAudio/Events/Default_Work_Unit/Fire_Alarm.Fire_Alarm" _returnvalue "0, 0, 0"))

(event Custom|SpawnSparks
  (bind _alarm (Variables|Default|GetAlarm))
  (bind _returnvalue (Transformation|GetWorldLocation _alarm))
  ;[1 1 1] Particle Events
  (Effects|SpawnEmitteratLocation "/Game/FPS/Textures/Effects/WeaponEffects/P_ImpactModified.P_ImpactModified" _returnvalue "0, 0, 0" "0.500000,0.500000,0.500000")
  (Class|AkGameplayStatics|PostEventatLocation "/Game/WwiseAudio/Events/Default_Work_Unit/Sparks.Sparks" _returnvalue "0, 0, 0"))

(event EventInteract
  (params (Instigator :type Actor%20Object%20Reference))
  ;[1 1 1] Server
  (if (not (Variables|Default|GetHasBeenInteractedWith))
    (CallFunction|MulticastInteract)
    (Variables|Default|SetHasBeenInteractedWith true)))

(event EventTick
  (params (DeltaSeconds :type Float%20%28single-precision%29))
  ;[1 1 1] Lerp To FallPointLocalPosition
  (if (and (< (Variables|Default|GetCurrentTimeTillFallen) (Variables|Default|GetTimeToFall)) (Variables|Default|GetIsFalling))
    (Variables|Default|SetCurrentFallSpeed (Math|Float|Clamp(Float) (+ (Variables|Default|GetCurrentFallSpeed) (* DeltaSeconds (Variables|Default|GetFallSpeedAcceleration))) 0.0 (Variables|Default|GetMaxFallSpeed)))
    (bind _output_get (Variables|Default|SetCurrentTimeTillFallen (Math|Float|Clamp(Float) (+ (Variables|Default|GetCurrentTimeTillFallen) (* (Variables|Default|GetCurrentFallSpeed) DeltaSeconds)) 0.0 (Variables|Default|GetTimeToFall))))
    (bind _output (CallFunction|Fitto01 _output_get (Variables|Default|GetTimeToFall)))
    (Transformation|SetRelativeLocation (Variables|Default|GetAlarm) (Math|Vector|Lerp(Vector) "0, 0, 0" (Variables|Default|GetFallPointLocalPosition) _output) false false)
    (bind _output_2 (CallFunction|Approximately (Variables|Default|GetCurrentTimeTillFallen) (Variables|Default|GetTimeToFall) 0.01))
    (if _output_2
      (if (Variables|Default|GetFireSpawned)
        _
        (else
          (Utilities|FlowControl|Delay 1.0)
          (CallFunction|SpawnFire)
          (Variables|Default|SetFireSpawned true)))
      (Networking|SwitchHasAuthority ; Only the server can change Replicated variables
        (:Authority
          (if (not (Variables|Default|GetAnimationComplete))
            (Variables|Default|SetAnimationComplete true)))))))

(fn ConstructionScript
  (Transformation|SetRelativeLocation (Variables|Default|GetFallPoint) (Variables|Default|GetFallPointLocalPosition) false false))

(fn OnRepAnimationComplete
  (CallFunction|OnRepAnimationCompleteEvent))

(fn BeginHover
  (params (Instigator :type Actor%20Object%20Reference))
  (return false))