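; BP_Britta_A is a child character class Blueprint for Britta, with leftover logic for a timed sprint class skill.
; The skill logic (run speed boost, sound, two-second reset, cooldown timer reported to the gameplay widget) is disconnected and never runs.
; UseClassSkill, Server and ResetCanUseSkill are empty; only the parent BeginPlay and construction calls, plus ServerResetRun's restore of default run speed, remain wired.
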(event Custom|Server
  ;[0.8079 1 0.4961] Class Skill
)

(event Custom|ServerResetRun
  ;[0.8079 1 0.4961] Class Skill
  (Variables|Default|SetRunSpeedModifier (Variables|Default|GetDefaultRunSpeedModdifier)))

(event Custom|ResetCanUseSkill)

(event EventBeginPlay
  (|CallParentFunction))

(event Collision|EventActorBeginOverlap
  (params (OtherActor :type Actor%20Object%20Reference)))

(event EventUseClassSkill
  ;[0.8079 1 0.4961] Class Skill
)

(fn ConstructionScript
  (|CallParentFunction))