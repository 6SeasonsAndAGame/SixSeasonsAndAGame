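; BP_Impact is an actor with a cube that plays a material-driven impact effect when a BP_Bullet hits it.
; On BeginPlay it creates a dynamic material instance on the cube.
; Each bullet hit writes the impact point to the material's Location parameter and restarts a timeline that animates the Amount parameter.
; A DestroyActor node is present but unconnected.
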(event OnComponentHit(Cube)
  (params (HitComponent :type Primitive%20Component%20Object%20Reference) (OtherActor :type Actor%20Object%20Reference) (OtherComp :type Primitive%20Component%20Object%20Reference) (NormalImpulse :type Vector :default "0, 0, 0") (Hit :type Hit%20Result%20Structure%20%28by%20ref%29))
  (bind _dyn_mat (Variables|Default|GetDyn_mat))
  (Utilities|Casting|CastToBP_Bullet OtherActor)
  (Rendering|Material|SetVectorParameterValue _dyn_mat "Location" (Math|Conversions|ToLinearColor(Vector) (.ImpactPoint (Collision|BreakHitResult Hit))) :!class /Script/Engine.MaterialInstanceDynamic)
  (bind _newtrack_0 (Timeline|Timeline_0 PlayFromStart)
    (:Update
      (Rendering|Material|SetScalarParameterValue _dyn_mat "Amount" _newtrack_0 :!class /Script/Engine.MaterialInstanceDynamic))))

(event EventBeginPlay
  (bind _returnvalue (Rendering|Material|CreateDynamicMaterialInstance (Variables|Default|GetCube) 0 0 "None" :!class /Script/Engine.PrimitiveComponent))
  (Variables|Default|SetDyn_mat _returnvalue))

(event Collision|EventActorBeginOverlap
  (params (OtherActor :type Actor%20Object%20Reference)))

(event EventTick
  (params (DeltaSeconds :type Float%20%28single-precision%29)))

(fn ConstructionScript)