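; BP_ACZone is a temporary hazard zone actor that damages zombies entering its box.
; On spawn it attaches the P_BlowDetails particle effect to the box, posts an audio event at its location, and destroys itself after a fixed delay.
; Each BP_Zombie that begins overlapping the box has CallZombieCount called on it, then receives damage once per overlap, with no ticking damage while inside.
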(event OnComponentBeginOverlap(Box)
  (params (OverlappedComponent :type Primitive%20Component%20Object%20Reference) (OtherActor :type Actor%20Object%20Reference) (OtherComp :type Primitive%20Component%20Object%20Reference) (OtherBodyIndex :type Integer) (bFromSweep :type Boolean) (SweepResult :type Hit%20Result%20Structure%20%28by%20ref%29))
  (bind _asbp_zombie (Utilities|Casting|CastToBP_Zombie OtherActor))
  (Default|CallZombieCount _asbp_zombie)
  (Game|Damage|ApplyDamage _asbp_zombie 1.0 0 0))

(event EventBeginPlay
  (bind _box (Variables|Default|GetBox))
  (Effects|SpawnEmitterAttached "/Game/FPS/Textures/Effects/Particles/Snow/P_BlowDetails.P_BlowDetails" _box "None" (Transformation|GetWorldLocation _box) "0, 0, 0" "1.000000,1.000000,1.000000" "KeepWorldPosition")
  (Class|AkGameplayStatics|PostEventatLocation 0 (Transformation|GetActorLocation self) "0, 0, 0")
  (Utilities|FlowControl|Delay 3e+01)
  (Actor|DestroyActor))

(fn ConstructionScript)