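; BP_Director is a zombie director that tracks living zombies and handles horde spawn requests up to a population cap.
; On BeginPlay it registers existing BP_Zombie and BP_HordeSpawner actors, binding to their kill and spawn-request events.
; Spawn requests are clamped to MaxZombies, placing each zombie at a random navmesh-reachable point near the requested location and registering it.
; Tick prints the current zombie count as a debug readout.
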(event EventBeginPlay
  (Utilities|FlowControl|Sequence
    (:then_0
      (bind _outactors (Actor|GetAllActorsOfClass "/Game/Zombies/ZBluePrints/BP_Zombie.BP_Zombie_C"))
      (for _array_element _outactors
        (Private|OnZombieSpawn _array_element)))
    (:then_1
      (bind _outactors_2 (Actor|GetAllActorsOfClass "/Game/Zombies/ZBluePrints/BP_HordeSpawner.BP_HordeSpawner_C"))
      (for _array_element_2 _outactors_2
        (Private|OnHordeSpawnerSpawned _array_element_2)))))

(event EventTick
  (params (DeltaSeconds :type Float%20%28single-precision%29))
  (Development|PrintString (Utilities|String|Append "Num Zombies: " (Utilities|String|ToString(Integer) (Utilities|Array|Length (Variables|Default|GetZombies)))) true true "(R=0.000000,G=0.660000,B=1.000000,A=1.000000)" 0.0))

(fn ConstructionScript)

(fn OnZombieSpawn
  (params (Zombie :type BP%20Zombie%20Object%20Reference))
  (Utilities|Array|Add (Variables|Default|GetZombies) Zombie)
  (EventDispatchers|BindEventtoOnKilled Zombie (EventDispatchers|CreateEvent :!event OnZombieKilled)))

(fn OnZombieKilled
  (params (Zombie :type BP%20Zombie%20Object%20Reference))
  (Utilities|Array|RemoveItem (Variables|Default|GetZombies) Zombie))

(fn OnHordeSpawnerSpawned
  (params (HordeSpawner :type BP%20Horde%20Spawner%20Object%20Reference))
  (Utilities|Array|Add (Variables|Default|GetHordSpawners) HordeSpawner)
  (EventDispatchers|BindEventtoRequestSpawn HordeSpawner (EventDispatchers|CreateEvent :!event OnZombieSpawnRequested)))

(fn OnZombieSpawnRequested
  (params (Count :type Integer) (Location :type Vector))
  (for _index (range 1 (Math|Integer|Min(Integer) Count (- (Variables|Default|GetMaxZombies) (Utilities|Array|Length (Variables|Default|GetZombies)))))
    (bind _returnvalue (Game|SpawnActorfromClass "/Game/Zombies/ZBluePrints/BP_Zombie.BP_Zombie_C" (Math|Transform|MakeTransform (+ (.RandomLocation (AI|Navigation|GetRandomReachablePointinRadius Location 5e+02 0 0)) "0, 0,88.000000") "0, 0, 0" "1,1,1") "AdjustIfPossibleButDontSpawnIfColliding" 0 "Bot" 0))
    (Utilities|IsValid _returnvalue
      (:Is%20Valid
        (Private|OnZombieSpawn _returnvalue)))))