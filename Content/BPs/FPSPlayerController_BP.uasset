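; FPSPlayerController_BP is a player controller that creates and updates the player's HUD.
; On BeginPlay it calls client-named events that add a HUD widget to the viewport, set game-only input, and refresh the team display.
; The refresh reads Team from TDPlayerState_BP and passes it to the HUD widget.
; CreateUI and UpdateUI events forward to the same client events.
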(event Custom|ClientCreateUI
  (bind _returnvalue (UserInterface|CreateWidget "/Game/WidgetBP/Menus/HUD/HUDUI_WB.HUDUI_WB_C"))
  (UserInterface|Viewport|AddtoViewport _returnvalue 0)
  (Input|SetInputModeGameOnly self))

(event Custom|ClientUpdateUI
  (bind _astdplayer_state_bp (Utilities|Casting|CastToTDPlayerState_BP (Variables|Default|GetPlayerState)))
  (Default|UpdateTeam (Variables|Default|GetHUD_Widget) (Variables|/Script/CTG.TDPlayerState|GetTeam _astdplayer_state_bp)))

(event EventBeginPlay
  (CallFunction|ClientCreateUI)
  (CallFunction|ClientUpdateUI))

(event EventTick
  (params (DeltaSeconds :type Float%20%28single-precision%29)))

(event EventUpdateUI
  (CallFunction|ClientUpdateUI))

(event EventCreateUI
  (CallFunction|ClientCreateUI))

(fn ConstructionScript)